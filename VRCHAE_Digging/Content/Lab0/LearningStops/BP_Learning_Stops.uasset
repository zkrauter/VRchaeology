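; Runs the VR lab's learning stops, spawning four numbered POIs, a front desk POI and a crate spawner.
; POIOverlap records which POI the VRPawn overlaps, and ActivateStop runs that stop's audio event, allowing one at a time.
; Numbered stops hide each other while active, then retire themselves and reveal unfinished ones, although Stop 4 never sets its finished flag.
; Stop 3 polls until all excavation tool flags are set before completing.
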(event Custom|Stop%203%20Loop
  (bind _stop3 (Variables|Default|GetStop3))
  ;[1 1 1] Comment
  (Utilities|FlowControl|Delay 0.1)
  (if (Math|Boolean|ANDBoolean (Variables|Default|GetbTrowelUsed) (Variables|Default|GetbSmallBrushUsed) (Variables|Default|GetbLargeBrushUsed) (Variables|Default|GetbTapeMeasureUsed) (Variables|Default|GetbStringUsed) (Variables|Default|GetbLevelUsed) (Variables|Default|GetbFlashlightUsed))
    (Variables|Default|SetbAllToolsUsed true)
    (Development|PrintString "All tools have been used (Trowel, Small Brush, Large Brush, Flashlight)"))
  (if (Variables|Default|GetbAllToolsUsed)
    (Utilities|FlowControl|Delay 1e+01)
    (Variables|Default|SetCurrentStop -1.0)
    (Variables|Default|SetbIsStopActive false)
    (if (Variables|Default|GetbStop1Finished)
      _
      (else
        (Rendering|SetActorHiddenInGame (Variables|Default|GetStop1) false)))
    (if (Variables|Default|GetbStop2Finished)
      _
      (else
        (Rendering|SetActorHiddenInGame (Variables|Default|GetStop2) false)))
    (if (Variables|Default|GetbStop4Finished)
      _
      (else
        (Rendering|SetActorHiddenInGame (Variables|Default|GetStop4) false)))
    (Rendering|SetActorHiddenInGame _stop3 true)
    (Collision|SetCollisionEnabled (Variables|/Game/Digging/Points_Of_Interest/BP_POI.BP_POI_C|GetGlowLightTriggerRadius _stop3) "NoCollision")
    (Variables|Default|SetbStop3Finished true)
    (Development|PrintString "- - - - - - - - - - - - - - - -")
    (else
      (CallFunction|Stop3Loop))))

(event Custom|POI%20Overlap
  ;[1 1 1] POI Overlap Check
  (Utilities|FlowControl|Sequence ; Checks what Stop we are overlapping
    (:then_0
      (bind _returnvalue (Actor|GetActorOfClass "/Game/VRTemplate/Blueprints/VRPawn.VRPawn_C")) ; Overlapping Stop 1
      (if (Collision|IsOverlappingActor (Variables|/Game/Digging/Points_Of_Interest/BP_POI.BP_POI_C|GetGlowLightTriggerRadius (Variables|Default|GetStop1)) _returnvalue :!class /Script/Engine.PrimitiveComponent)
        (bind _output_get (Variables|Default|SetCurrentStop 1.0))
        (Development|PrintString "Stop 1 overlap actor")
        (Development|PrintString (Utilities|String|ToString(Float) _output_get))))
    (:then_1
      (bind _returnvalue_2 (Actor|GetActorOfClass "/Game/VRTemplate/Blueprints/VRPawn.VRPawn_C")) ; Overlapping Stop 2
      (if (Collision|IsOverlappingActor (Variables|/Game/Digging/Points_Of_Interest/BP_POI.BP_POI_C|GetGlowLightTriggerRadius (Variables|Default|GetStop2)) _returnvalue_2 :!class /Script/Engine.PrimitiveComponent)
        (bind _output_get_2 (Variables|Default|SetCurrentStop 2.0))
        (Development|PrintString "Stop 2 overlap actor")
        (Development|PrintString (Utilities|String|ToString(Float) _output_get_2))))
    (:then_2
      (bind _returnvalue_3 (Actor|GetActorOfClass "/Game/VRTemplate/Blueprints/VRPawn.VRPawn_C")) ; Overlapping Stop 3
      (if (Collision|IsOverlappingActor (Variables|/Game/Digging/Points_Of_Interest/BP_POI.BP_POI_C|GetGlowLightTriggerRadius (Variables|Default|GetStop3)) _returnvalue_3 :!class /Script/Engine.PrimitiveComponent)
        (bind _output_get_3 (Variables|Default|SetCurrentStop 3.0))
        (Development|PrintString "Stop 3 overlap actor")
        (Development|PrintString (Utilities|String|ToString(Float) _output_get_3))))
    (:then_3
      (bind _returnvalue_4 (Actor|GetActorOfClass "/Game/VRTemplate/Blueprints/VRPawn.VRPawn_C")) ; Overlapping Stop 4
      (if (Collision|IsOverlappingActor (Variables|/Game/Digging/Points_Of_Interest/BP_POI.BP_POI_C|GetGlowLightTriggerRadius (Variables|Default|GetStop4)) _returnvalue_4 :!class /Script/Engine.PrimitiveComponent)
        (bind _output_get_4 (Variables|Default|SetCurrentStop 4.0))
        (Development|PrintString "Stop 4 overlap actor")
        (Development|PrintString (Utilities|String|ToString(Float) _output_get_4))))
    (:then_4
      (bind _returnvalue_5 (Actor|GetActorOfClass "/Game/VRTemplate/Blueprints/VRPawn.VRPawn_C"))
      (if (Collision|IsOverlappingActor (Variables|/Game/Digging/Points_Of_Interest/BP_POI.BP_POI_C|GetGlowLightTriggerRadius (Variables|Default|GetFrontDeskStop)) _returnvalue_5 :!class /Script/Engine.PrimitiveComponent)
        (bind _output_get_5 (Variables|Default|SetCurrentStop 5.0))
        (Development|PrintString "FrontDesk Overlap")
        (Development|PrintString (Utilities|String|ToString(Float) _output_get_5))))))

(event Custom|Front%20Desk%20Event
  ;[1 1 1] Comment
  (Audio|PlaySound2D "/Game/VRCH_tutorial_voiceovers/polly_phonecall_1.polly_phonecall_1" 1.0 1.0 0.0 0 0)
  (Development|PrintString "Front desk sound done, now delaying")
  (Utilities|FlowControl|Delay 5.0)
  (Variables|Default|SetCurrentStop -1.0)
  (Variables|Default|SetbIsStopActive false)
  (Development|PrintString "- - - - - - - - - - - - - - - -"))

(event Custom|Stop%201%20Event
  (bind _stop1 (Variables|Default|GetStop1))
  ;[1 1 1] Comment
  (Audio|PlaySound2D "/Game/VRCH_tutorial_voiceovers/stop_1.stop_1" 1.0 1.0 0.0 0 0)
  (Utilities|FlowControl|Delay 1e+01)
  (Variables|Default|SetCurrentStop -1.0)
  (Variables|Default|SetbIsStopActive false)
  (if (Variables|Default|GetbStop2Finished)
    _
    (else
      (Rendering|SetActorHiddenInGame (Variables|Default|GetStop2) false)))
  (if (Variables|Default|GetbStop3Finished)
    _
    (else
      (Rendering|SetActorHiddenInGame (Variables|Default|GetStop3) false)))
  (if (Variables|Default|GetbStop4Finished)
    _
    (else
      (Rendering|SetActorHiddenInGame (Variables|Default|GetStop4) false)))
  (Rendering|SetActorHiddenInGame _stop1 true)
  (Collision|SetCollisionEnabled (Variables|/Game/Digging/Points_Of_Interest/BP_POI.BP_POI_C|GetGlowLightTriggerRadius _stop1) "NoCollision")
  (Variables|Default|SetbStop1Finished true)
  (Development|PrintString "- - - - - - - - - - - - - - - -"))

(event Custom|Stop%202%20Event
  (bind _stop2 (Variables|Default|GetStop2))
  ;[1 1 1] Comment
  (Audio|PlaySound2D "/Game/VRCH_tutorial_voiceovers/artifact_repository_v2.artifact_repository_v2" 1.0 1.0 0.0 0 0)
  (Utilities|FlowControl|Delay 1e+01)
  (Variables|Default|SetCurrentStop -1.0)
  (Variables|Default|SetbIsStopActive false)
  (if (Variables|Default|GetbStop1Finished)
    _
    (else
      (Rendering|SetActorHiddenInGame (Variables|Default|GetStop1) false)))
  (if (Variables|Default|GetbStop3Finished)
    _
    (else
      (Rendering|SetActorHiddenInGame (Variables|Default|GetStop3) false)))
  (if (Variables|Default|GetbStop4Finished)
    _
    (else
      (Rendering|SetActorHiddenInGame (Variables|Default|GetStop4) false)))
  (Rendering|SetActorHiddenInGame _stop2 true)
  (Collision|SetCollisionEnabled (Variables|/Game/Digging/Points_Of_Interest/BP_POI.BP_POI_C|GetGlowLightTriggerRadius _stop2) "NoCollision")
  (Variables|Default|SetbStop2Finished true)
  (Development|PrintString "- - - - - - - - - - - - - - - -"))

(event Custom|Stop%203%20Event
  ;[1 1 1] Comment
  (CallFunction|Stop3Function)
  (CallFunction|Stop3Loop) ; This loop is needed since we need to constantly check if our conditions are true
)

(event Custom|Stop%204%20Event
  (bind _stop4 (Variables|Default|GetStop4))
  ;[1 1 1] Comment
  (Audio|PlaySound2D "/Game/VRCH_tutorial_voiceovers/broken_vase.broken_vase" 1.0 1.0 0.0 0 0)
  (Utilities|FlowControl|Delay 1e+01)
  (Variables|Default|SetCurrentStop -1.0)
  (Variables|Default|SetbIsStopActive false)
  (if (Variables|Default|GetbStop1Finished)
    _
    (else
      (Rendering|SetActorHiddenInGame (Variables|Default|GetStop1) false)))
  (if (Variables|Default|GetbStop2Finished)
    _
    (else
      (Rendering|SetActorHiddenInGame (Variables|Default|GetStop2) false)))
  (if (Variables|Default|GetbStop3Finished)
    _
    (else
      (Rendering|SetActorHiddenInGame (Variables|Default|GetStop3) false)))
  (Rendering|SetActorHiddenInGame _stop4 true)
  (Collision|SetCollisionEnabled (Variables|/Game/Digging/Points_Of_Interest/BP_POI.BP_POI_C|GetGlowLightTriggerRadius _stop4) "NoCollision")
  (Variables|Default|SetbStop4Finished false)
  (Development|PrintString "- - - - - - - - - - - - - - - -"))

(event EventBeginPlay
  (bind _returnvalue (Game|SpawnActorfromClass "/Game/Digging/Points_Of_Interest/BP_POI.BP_POI_C" (Math|Transform|MakeTransform "488.000000,-168.000000,270.000000" "0, 0, 0" "1.000000,1.000000,1.000000") "Undefined" "MultiplyWithRoot" 0 0)) ; Front Desk Stop
  (Variables|Default|SetFrontDeskStop _returnvalue)
  (bind _returnvalue_2 (Game|SpawnActorfromClass "/Game/Digging/Points_Of_Interest/BP_POI.BP_POI_C" (Math|Transform|MakeTransform "77.373008,-349.268255,319.588437" "0, 0, 0" "1.000000,1.000000,1.000000") "Undefined" "MultiplyWithRoot" 0 0)) ; Stop 1
  (Variables|Default|SetStop1 _returnvalue_2)
  (bind _returnvalue_3 (Game|SpawnActorfromClass "/Game/Digging/Points_Of_Interest/BP_POI.BP_POI_C" (Math|Transform|MakeTransform "237.962074,-667.338410,300.512656" "0, 0, 0" "1.000000,1.000000,1.000000") "Undefined" "MultiplyWithRoot" 0 0)) ; Stop 2
  (Variables|Default|SetStop2 _returnvalue_3)
  (bind _returnvalue_4 (Game|SpawnActorfromClass "/Game/Digging/Points_Of_Interest/BP_POI.BP_POI_C" (Math|Transform|MakeTransform "484.865230,-515.779131,297.886436" "0, 0, 0" "1.000000,1.000000,1.000000") "Undefined" "MultiplyWithRoot" 0 0)) ; Stop 3
  (Variables|Default|SetStop3 _returnvalue_4)
  (bind _returnvalue_5 (Game|SpawnActorfromClass "/Game/Digging/Points_Of_Interest/BP_POI.BP_POI_C" (Math|Transform|MakeTransform "890.986437,-358.536229,303.145322" "0, 0, 0" "1.000000,1.000000,1.000000") "Undefined" "MultiplyWithRoot" 0 0)) ; Stop 4
  (Variables|Default|SetStop4 _returnvalue_5)
  (bind _returnvalue_6 (Game|SpawnActorfromClass "/Game/Digging/Ground/BP_BlockSpawner.BP_BlockSpawner_C" (Math|Transform|MakeTransform "0, 0, 0" "0, 0, 0" "1.000000,1.000000,1.000000") "Undefined" "MultiplyWithRoot" 0 0))
  (Default|Level0CrateSpawner _returnvalue_6))

(event EventTick
  (params (DeltaSeconds :type Float%20%28single-precision%29)))

(fn ConstructionScript)

(fn ActivateStop
  (bind _currentstop (Variables|Default|GetCurrentStop))
  (if (Variables|Default|GetbIsStopActive) ; Only activate a Stop when none are active
    (Development|PrintString "A Stop is already underway!")
    (else
      (Variables|Default|SetbIsStopActive true)
      (Development|PrintString "Entering the \"Switch\" logic")
      (Development|PrintString (Utilities|String|ToString(Float) _currentstop))
      (switch int (Math|Float|Truncate _currentstop) ; Hides other Stops, depending on what Stop is active
        (:1
          (Rendering|SetActorHiddenInGame (Variables|Default|GetStop2) true)
          (Rendering|SetActorHiddenInGame (Variables|Default|GetStop3) true)
          (Rendering|SetActorHiddenInGame (Variables|Default|GetStop4) true)
          (Development|PrintString "Time to run Stop 1")
          (CallFunction|Stop1Event))
        (:2
          (Rendering|SetActorHiddenInGame (Variables|Default|GetStop1) true)
          (Rendering|SetActorHiddenInGame (Variables|Default|GetStop3) true)
          (Rendering|SetActorHiddenInGame (Variables|Default|GetStop4) true)
          (Development|PrintString "Time to run Stop 2")
          (CallFunction|Stop2Event))
        (:3
          (Rendering|SetActorHiddenInGame (Variables|Default|GetStop1) true)
          (Rendering|SetActorHiddenInGame (Variables|Default|GetStop2) true)
          (Rendering|SetActorHiddenInGame (Variables|Default|GetStop4) true)
          (Development|PrintString "Time to run Stop 3")
          (CallFunction|Stop3Event))
        (:4
          (Rendering|SetActorHiddenInGame (Variables|Default|GetStop1) true)
          (Rendering|SetActorHiddenInGame (Variables|Default|GetStop2) true)
          (Rendering|SetActorHiddenInGame (Variables|Default|GetStop3) true)
          (Development|PrintString "Time to run Stop 4")
          (CallFunction|Stop4Event))
        (:5
          (CallFunction|FrontDeskEvent))))))

(fn Stop1Function)

(fn Stop2Function)

(fn Stop3Function
  (Audio|PlaySound2D "/Game/VRCH_tutorial_voiceovers/sandbox.sandbox" 1.0 1.0 0.0 0 0)
  (if (Math|Boolean|ANDBoolean (Variables|Default|GetbTrowelUsed) (Variables|Default|GetbSmallBrushUsed) (Variables|Default|GetbLargeBrushUsed) (Variables|Default|GetbTapeMeasureUsed) (Variables|Default|GetbStringUsed) (Variables|Default|GetbLevelUsed) (Variables|Default|GetbFlashlightUsed))
    (Variables|Default|SetbAllToolsUsed true)
    (Development|PrintString "All tools have been used")))

(fn Stop4Function)