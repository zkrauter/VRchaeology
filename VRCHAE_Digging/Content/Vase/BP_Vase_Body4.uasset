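; BP_Vase_Body4 is one fragment of a vase assembly puzzle, to which neighboring pieces snap on contact.
; Once it is itself attached, its Sphere overlap casts the other actor to Neck3, Neck1, Body5 or Body_2.
; A matching piece is attached to Body4 with snap rules, flagged as attached and set to Static mobility, so attachment can propagate piece by piece.
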(event OnComponentBeginOverlap(Sphere)
  (params (OverlappedComponent :type Primitive%20Component%20Object%20Reference) (OtherActor :type Actor%20Object%20Reference) (OtherComp :type Primitive%20Component%20Object%20Reference) (OtherBodyIndex :type Integer) (bFromSweep :type Boolean) (SweepResult :type Hit%20Result%20Structure%20%28by%20ref%29))
  ;[1 1 1] If any of the parts that stick with Body4 come in contact with Body4 they would snap and bind to Body 4, see Base2 Blueprint for more specific details (Note all blueprints are identical)
  (if (Variables|Default|GetisBody4Attached)
    (bind _asbp_vase_neck_3 (Utilities|Casting|CastToBP_Vase_Neck3 OtherActor)
      (:then
        (Transformation|AttachComponentToComponent (Variables|/Script/Engine.Actor|GetRootComponent _asbp_vase_neck_3) (Variables|Default|GetBody4) "None" "SnapToTarget" "SnapToTarget" "SnapToTarget" true)
        (Variables|/Game/Vase/BP_Vase_Neck3.BP_Vase_Neck3_C|SetisNeck3Attached _asbp_vase_neck_3 true)
        (Transformation|SetMobility (Variables|/Script/Engine.Actor|GetRootComponent _asbp_vase_neck_3) "Static"))
      (:CastFailed
        (bind _asbp_vase_neck_1 (Utilities|Casting|CastToBP_Vase_Neck1 OtherActor)
          (:then
            (Transformation|AttachComponentToComponent (Variables|/Script/Engine.Actor|GetRootComponent _asbp_vase_neck_1) (Variables|Default|GetBody4) "None" "SnapToTarget" "SnapToTarget" "SnapToTarget" true)
            (Variables|/Game/Vase/BP_Vase_Neck1.BP_Vase_Neck1_C|SetisNeck1Attached _asbp_vase_neck_1 true)
            (Transformation|SetMobility (Variables|/Script/Engine.Actor|GetRootComponent _asbp_vase_neck_1) "Static"))
          (:CastFailed
            (bind _asbp_vase_body_5 (Utilities|Casting|CastToBP_Vase_Body5 OtherActor)
              (:then
                (Transformation|AttachComponentToComponent (Variables|/Script/Engine.Actor|GetRootComponent _asbp_vase_body_5) (Variables|Default|GetBody4) "None" "SnapToTarget" "SnapToTarget" "SnapToTarget" true)
                (Variables|/Game/Vase/BP_Vase_Body5.BP_Vase_Body5_C|SetisBody5Attached _asbp_vase_body_5 true)
                (Transformation|SetMobility (Variables|/Script/Engine.Actor|GetRootComponent _asbp_vase_body_5) "Static"))
              (:CastFailed
                (bind _asbp_vase_body_2 (Utilities|Casting|CastToBP_Vase_Body_2 OtherActor))
                (Transformation|AttachComponentToComponent (Variables|/Script/Engine.Actor|GetRootComponent _asbp_vase_body_2) (Variables|Default|GetBody4) "None" "SnapToTarget" "SnapToTarget" "SnapToTarget" true)
                (Variables|/Game/Vase/BP_Vase_Body_2.BP_Vase_Body_2_C|SetisBody2Attached _asbp_vase_body_2 true)
                (Transformation|SetMobility (Variables|/Script/Engine.Actor|GetRootComponent _asbp_vase_body_2) "Static")))))))))

(fn ConstructionScript)