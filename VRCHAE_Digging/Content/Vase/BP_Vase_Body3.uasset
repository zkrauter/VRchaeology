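; BP_Vase_Body3 is one piece of a vase assembly that snaps neighboring pieces onto itself.
; When its Sphere overlaps Body2 or Body5 while Body3 is itself attached, it snap-attaches that piece's root to Body3, flags it as attached and makes it static.
; The attached flag gates the chain, so pieces only bind onto already-assembled parts, following a pattern shared with the other vase part Blueprints.
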(event OnComponentBeginOverlap(Sphere)
  (params (OverlappedComponent :type Primitive%20Component%20Object%20Reference) (OtherActor :type Actor%20Object%20Reference) (OtherComp :type Primitive%20Component%20Object%20Reference) (OtherBodyIndex :type Integer) (bFromSweep :type Boolean) (SweepResult :type Hit%20Result%20Structure%20%28by%20ref%29))
  ;[1 1 1] If any of the parts that stick with Body3 come in contact with Body3 they would snap and bind to Body3, see Base2 Blueprint for more specific details of all the blocks in the blueprint (Note all blueprints are similar)
  (if (Variables|Default|GetisBody3Attached)
    (bind _asbp_vase_body_2 (Utilities|Casting|CastToBP_Vase_Body_2 OtherActor)
      (:then
        (Transformation|AttachComponentToComponent (Variables|/Script/Engine.Actor|GetRootComponent _asbp_vase_body_2) (Variables|Default|GetBody3) "None" "SnapToTarget" "SnapToTarget" "SnapToTarget" true)
        (Variables|/Game/Vase/BP_Vase_Body_2.BP_Vase_Body_2_C|SetisBody2Attached _asbp_vase_body_2 true)
        (Transformation|SetMobility (Variables|/Script/Engine.Actor|GetRootComponent _asbp_vase_body_2) "Static"))
      (:CastFailed
        (bind _asbp_vase_body_5 (Utilities|Casting|CastToBP_Vase_Body5 OtherActor))
        (Transformation|AttachComponentToComponent (Variables|/Script/Engine.Actor|GetRootComponent _asbp_vase_body_5) (Variables|Default|GetBody3) "None" "SnapToTarget" "SnapToTarget" "SnapToTarget" true)
        (Variables|/Game/Vase/BP_Vase_Body5.BP_Vase_Body5_C|SetisBody5Attached _asbp_vase_body_5 true)
        (Transformation|SetMobility (Variables|/Script/Engine.Actor|GetRootComponent _asbp_vase_body_5) "Static")))))

(fn ConstructionScript)

(fn NewFunction
  (params (NewParam :type Boolean) (NewParam1 :type Boolean)))