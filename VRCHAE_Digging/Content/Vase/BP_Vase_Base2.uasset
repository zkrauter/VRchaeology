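; BP_Vase_Base2 is the Base2 piece of a breakable-vase assembly that neighbouring fragments snap onto.
; When its overlap sphere touches Body1, Base1, Body3 or Body6, a cast chain identifies the piece and attaches its root to Base2 with snap-to-target transforms.
; The attached piece gets its own attached flag set and its mobility switched to Static, locking it in place.
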(event OnComponentBeginOverlap(SphereCollisionBase2)
  (params (OverlappedComponent :type Primitive%20Component%20Object%20Reference) (OtherActor :type Actor%20Object%20Reference) (OtherComp :type Primitive%20Component%20Object%20Reference) (OtherBodyIndex :type Integer) (bFromSweep :type Boolean) (SweepResult :type Hit%20Result%20Structure%20%28by%20ref%29))
  ;[1 1 1] If any of the parts that stick with Base2 come in contact with Base2 they would snap and bind to Base2
  (bind _asbp_vase_body_1 (Utilities|Casting|CastToBP_Vase_Body1 OtherActor)
    (:then
      (Transformation|AttachComponentToComponent (Variables|/Script/Engine.Actor|GetRootComponent _asbp_vase_body_1) (Variables|Default|GetBase2) "None" "SnapToTarget" "SnapToTarget" "SnapToTarget" true)
      (Variables|/Game/Vase/BP_Vase_Body1.BP_Vase_Body1_C|SetisBody1Attached _asbp_vase_body_1 true)
      (Transformation|SetMobility (Variables|/Script/Engine.Actor|GetRootComponent _asbp_vase_body_1) "Static"))
    (:CastFailed
      (bind _asbp_vase_base_1 (Utilities|Casting|CastToBP_Vase_Base1 OtherActor)
        (:then
          (Transformation|AttachComponentToComponent (Variables|/Script/Engine.Actor|GetRootComponent _asbp_vase_base_1) (Variables|Default|GetBase2) "None" "SnapToTarget" "SnapToTarget" "SnapToTarget" true)
          (Variables|/Game/Vase/BP_Vase_Base1.BP_Vase_Base1_C|SetisBase1Attached _asbp_vase_base_1 true)
          (Transformation|SetMobility (Variables|/Script/Engine.Actor|GetRootComponent _asbp_vase_base_1) "Static"))
        (:CastFailed
          (bind _asbp_vase_body_3 (Utilities|Casting|CastToBP_Vase_Body3 OtherActor)
            (:then
              (Transformation|AttachComponentToComponent (Variables|/Script/Engine.Actor|GetRootComponent _asbp_vase_body_3) (Variables|Default|GetBase2) "None" "SnapToTarget" "SnapToTarget" "SnapToTarget" true)
              (Variables|/Game/Vase/BP_Vase_Body3.BP_Vase_Body3_C|SetisBody3Attached _asbp_vase_body_3 true)
              (Transformation|SetMobility (Variables|/Script/Engine.Actor|GetRootComponent _asbp_vase_body_3) "Static"))
            (:CastFailed
              (bind _asbp_vase_body_6 (Utilities|Casting|CastToBP_Vase_Body6 OtherActor))
              (Transformation|AttachComponentToComponent (Variables|/Script/Engine.Actor|GetRootComponent _asbp_vase_body_6) (Variables|Default|GetBase2) "None" "SnapToTarget" "SnapToTarget" "SnapToTarget" true)
              (Variables|/Game/Vase/BP_Vase_Body6.BP_Vase_Body6_C|SetisBody6Attached _asbp_vase_body_6 true)
              (Transformation|SetMobility (Variables|/Script/Engine.Actor|GetRootComponent _asbp_vase_body_6) "Static"))))))))

(fn ConstructionScript)