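; BP_Vase_Part is a grabbable vase piece, apparently intended to join a vase assembly.
; The construction script applies the configured mesh and sets the position and radius of its overlap sphere.
; Grabbing sets IsGrabbedChild.
; The overlap event is empty, leaving the logic that casts to BP_Vase_Base2, snap-attaches and makes it static disconnected; a note says it conflicts with BP_Vase_Parent's logic.
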(event OnComponentBeginOverlap(SphereCollisionChild)
  (params (OverlappedComponent :type Primitive%20Component%20Object%20Reference) (OtherActor :type Actor%20Object%20Reference) (OtherComp :type Primitive%20Component%20Object%20Reference) (OtherBodyIndex :type Integer) (bFromSweep :type Boolean) (SweepResult :type Hit%20Result%20Structure%20%28by%20ref%29))
  ;[1 1 1] This code fixes the issue off BP_Vase_Part not being able to stick to BP_Vase_Parent, when the BP_Vase_Part is brought to the parent. However, the blueprint in BP_Vase_Parent can't be running while this is running
)

(event OnGrabbed(GrabComponentChild)
  ;[1 1 1] This code fixes the issue off BP_Vase_Part not being able to stick to BP_Vase_Parent, when the BP_Vase_Part is brought to the parent. However, the blueprint in BP_Vase_Parent can't be running while this is running
  (Variables|Default|SetIsGrabbedChild true))

(event EventBeginPlay)

(event Collision|EventActorBeginOverlap
  (params (OtherActor :type Actor%20Object%20Reference)))

(event EventTick
  (params (DeltaSeconds :type Float%20%28single-precision%29)))

(fn ConstructionScript
  (Components|StaticMesh|SetStaticMesh (Variables|Default|GetVasePart) (Variables|Default|GetMesh))
  (Transformation|SetRelativeLocation (Variables|Default|GetSphereCollisionChild) (Variables|Default|Getcollision_location) false true)
  (Components|Sphere|SetSphereRadius (Variables|Default|GetSphereCollisionChild) (Variables|Default|Getsize_collision) true))