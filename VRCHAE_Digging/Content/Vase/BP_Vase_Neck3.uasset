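; BP_Vase_Neck3 is the Neck3 piece of a vase assembled from parts that snap together on contact.
; When its Sphere overlaps an actor while IsNeck3Attached is true, a cast chain checks for the Neck2, Rim or Body4 Blueprint.
; A matching piece is snapped to Neck3, flagged as attached through its own boolean, and set to Static mobility.
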(event OnComponentBeginOverlap(Sphere)
  (params (OverlappedComponent :type Primitive%20Component%20Object%20Reference) (OtherActor :type Actor%20Object%20Reference) (OtherComp :type Primitive%20Component%20Object%20Reference) (OtherBodyIndex :type Integer) (bFromSweep :type Boolean) (SweepResult :type Hit%20Result%20Structure%20%28by%20ref%29))
  ;[1 1 1] If any of the parts that stick with Neck3 come in contact with Neck3 they would snap and bind to Neck3, see Base2 Blueprint for more specific details (Note all blueprints are identical)
  (if (Variables|Default|GetisNeck3Attached)
    (bind _asbp_vase_neck_2 (Utilities|Casting|CastToBP_Vase_Neck2 OtherActor)
      (:then
        (Transformation|AttachComponentToComponent (Variables|/Script/Engine.Actor|GetRootComponent _asbp_vase_neck_2) (Variables|Default|GetNeck3) "None" "SnapToTarget" "SnapToTarget" "SnapToTarget" true)
        (Variables|/Game/Vase/BP_Vase_Neck2.BP_Vase_Neck2_C|SetisNeck2Attached _asbp_vase_neck_2 true)
        (Transformation|SetMobility (Variables|/Script/Engine.Actor|GetRootComponent _asbp_vase_neck_2) "Static"))
      (:CastFailed
        (bind _asbp_vase_rim (Utilities|Casting|CastToBP_Vase_Rim OtherActor)
          (:then
            (Transformation|AttachComponentToComponent (Variables|/Script/Engine.Actor|GetRootComponent _asbp_vase_rim) (Variables|Default|GetNeck3) "None" "SnapToTarget" "SnapToTarget" "SnapToTarget" true)
            (Variables|/Game/Vase/BP_Vase_Rim.BP_Vase_Rim_C|SetisRimAttached _asbp_vase_rim true)
            (Transformation|SetMobility (Variables|/Script/Engine.Actor|GetRootComponent _asbp_vase_rim) "Static"))
          (:CastFailed
            (bind _asbp_vase_body_4 (Utilities|Casting|CastToBP_Vase_Body4 OtherActor))
            (Transformation|AttachComponentToComponent (Variables|/Script/Engine.Actor|GetRootComponent _asbp_vase_body_4) (Variables|Default|GetNeck3) "None" "SnapToTarget" "SnapToTarget" "SnapToTarget" true)
            (Variables|/Game/Vase/BP_Vase_Body4.BP_Vase_Body4_C|SetisBody4Attached _asbp_vase_body_4 true)
            (Transformation|SetMobility (Variables|/Script/Engine.Actor|GetRootComponent _asbp_vase_body_4) "Static")))))))

(fn ConstructionScript)