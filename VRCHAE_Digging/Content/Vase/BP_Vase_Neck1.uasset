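; BP_Vase_Neck1 is the first neck piece of a vase that assembles from snapping fragments.
; Once Neck1 is itself attached, its Sphere overlap runs a cast chain for Neck2, Neck3, Rim, Body5 and Body4 pieces.
; A matching piece snaps to the Neck1 component, gets its own attached flag set and becomes Static.
; That flag suggests attachment propagates piece by piece, with the same pattern in the sibling vase Blueprints.
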(event OnComponentBeginOverlap(Sphere)
  (params (OverlappedComponent :type Primitive%20Component%20Object%20Reference) (OtherActor :type Actor%20Object%20Reference) (OtherComp :type Primitive%20Component%20Object%20Reference) (OtherBodyIndex :type Integer) (bFromSweep :type Boolean) (SweepResult :type Hit%20Result%20Structure%20%28by%20ref%29))
  ;[1 1 1] If any of the parts that stick with Neck1 come in contact with Neck1 they would snap and bind to Neck1, see Base2 Blueprint for more specific details of all the blocks in the blueprint (Note all blueprints are similar)
  (if (Variables|Default|GetisNeck1Attached)
    (bind _asbp_vase_neck_2 (Utilities|Casting|CastToBP_Vase_Neck2 OtherActor)
      (:then
        (Transformation|AttachComponentToComponent (Variables|/Script/Engine.Actor|GetRootComponent _asbp_vase_neck_2) (Variables|Default|GetNeck1) "None" "SnapToTarget" "SnapToTarget" "SnapToTarget" true)
        (Variables|/Game/Vase/BP_Vase_Neck2.BP_Vase_Neck2_C|SetisNeck2Attached _asbp_vase_neck_2 true)
        (Transformation|SetMobility (Variables|/Script/Engine.Actor|GetRootComponent _asbp_vase_neck_2) "Static"))
      (:CastFailed
        (bind _asbp_vase_neck_3 (Utilities|Casting|CastToBP_Vase_Neck3 OtherActor)
          (:then
            (Transformation|AttachComponentToComponent (Variables|/Script/Engine.Actor|GetRootComponent _asbp_vase_neck_3) (Variables|Default|GetNeck1) "None" "SnapToTarget" "SnapToTarget" "SnapToTarget" true)
            (Variables|/Game/Vase/BP_Vase_Neck3.BP_Vase_Neck3_C|SetisNeck3Attached _asbp_vase_neck_3 true)
            (Transformation|SetMobility (Variables|/Script/Engine.Actor|GetRootComponent _asbp_vase_neck_3) "Static"))
          (:CastFailed
            (bind _asbp_vase_rim (Utilities|Casting|CastToBP_Vase_Rim OtherActor)
              (:then
                (Transformation|AttachComponentToComponent (Variables|/Script/Engine.Actor|GetRootComponent _asbp_vase_rim) (Variables|Default|GetNeck1) "None" "SnapToTarget" "SnapToTarget" "SnapToTarget" true)
                (Variables|/Game/Vase/BP_Vase_Rim.BP_Vase_Rim_C|SetisRimAttached _asbp_vase_rim true)
                (Transformation|SetMobility (Variables|/Script/Engine.Actor|GetRootComponent _asbp_vase_rim) "Static"))
              (:CastFailed
                (bind _asbp_vase_body_5 (Utilities|Casting|CastToBP_Vase_Body5 OtherActor)
                  (:then
                    (Transformation|AttachComponentToComponent (Variables|/Script/Engine.Actor|GetRootComponent _asbp_vase_body_5) (Variables|Default|GetNeck1) "None" "SnapToTarget" "SnapToTarget" "SnapToTarget" true)
                    (Variables|/Game/Vase/BP_Vase_Body5.BP_Vase_Body5_C|SetisBody5Attached _asbp_vase_body_5 true)
                    (Transformation|SetMobility (Variables|/Script/Engine.Actor|GetRootComponent _asbp_vase_body_5) "Static"))
                  (:CastFailed
                    (bind _asbp_vase_body_4 (Utilities|Casting|CastToBP_Vase_Body4 OtherActor))
                    (Transformation|AttachComponentToComponent (Variables|/Script/Engine.Actor|GetRootComponent _asbp_vase_body_4) (Variables|Default|GetNeck1) "None" "SnapToTarget" "SnapToTarget" "SnapToTarget" true)
                    (Variables|/Game/Vase/BP_Vase_Body4.BP_Vase_Body4_C|SetisBody4Attached _asbp_vase_body_4 true)
                    (Transformation|SetMobility (Variables|/Script/Engine.Actor|GetRootComponent _asbp_vase_body_4) "Static")))))))))))

(fn ConstructionScript)