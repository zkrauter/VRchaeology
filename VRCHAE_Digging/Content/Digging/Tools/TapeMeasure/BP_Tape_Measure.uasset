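; VR tape measure tool that measures from a start point to where its arrow points.
; With the tool attached to VRPawn, the right trigger records PointA and toggles a Tick gate that line-traces for PointB.
; Debug draws render the line, with scaled distance text at its midpoint, both lingering for DebugLineTimer after measuring stops.
; In Lab_0_Level, measuring also flags BP_Learning_Stops for the tutorial.
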(event Custom|TapeMeasureEvent
  ;[1 1 1] Old Stuff
)

(event Custom|Disappear
  (Rendering|Debug|DrawDebugLine (Variables|Default|GetPoint%20A) (Variables|Default|GetPoint%20B) "(R=1.000000,G=0.019947,B=0.059748,A=1.000000)" (Variables|Default|GetdebugLineTimer) 1.0)
  (Utilities|FlowControl|Delay (Variables|Default|GetdebugLineTimer))
  (Rendering|SetVisibility (Variables|Default|GetDistance) false false))

(event Input|EnhancedActionEvents|EnhancedInputActionIA_Right_Trigger
  (params (ActionValue :type Boolean) (ElapsedSeconds :type Float%20%28double-precision%29) (TriggeredSeconds :type Float%20%28double-precision%29) (InputAction :type Input%20Action%20Object%20Reference :default "/Game/VRTemplate/Input/Actions/IA_Right_Trigger.IA_Right_Trigger"))
  (bind _arrow (Variables|Default|GetArrow))
  (bind _distance (Variables|Default|GetDistance))
  (bind _returnvalue (Transformation|GetWorldLocation _arrow))
  (bind _returnvalue_2 (Actor|GetActorOfClass "/Game/VRTemplate/Blueprints/VRPawn.VRPawn_C")) ; Get the VRPawn to get the player hand.
  (if (Variables|/Game/VRTemplate/Blueprints/VRPawn.VRPawn_C|GetbIsTapeMeasureAttached _returnvalue_2)
    (if (Variables|Default|GetbIsMeasuring)
      (Variables|Default|SetbIsMeasuring false)
      (CallFunction|Disappear)
      (Utilities|FlowControl|Gate true) ; enters at Close
      (else
        (Rendering|Debug|FlushPersistentDebugLines)
        (Rendering|SetVisibility (Variables|Default|GetDistance) true false)
        (Variables|Default|SetbIsMeasuring true)
        (Variables|Default|SetPoint%20A (Transformation|GetWorldLocation (Variables|Default|GetArrow)))
        (Utilities|FlowControl|Gate true) ; enters at Open
      ))))

(event EventBeginPlay
  (Input|EnableInput (Game|GetPlayerController 0)))

(event Collision|EventActorBeginOverlap
  (params (OtherActor :type Actor%20Object%20Reference)))

(event EventTick
  (params (DeltaSeconds :type Float%20%28single-precision%29))
  (bind _point_a (Variables|Default|GetPoint%20A))
  (bind _arrow (Variables|Default|GetArrow))
  (bind _distance (Variables|Default|GetDistance))
  (bind _returnvalue (Transformation|GetWorldLocation _arrow))
  (Utilities|FlowControl|Gate true
    (:Exit
      (Utilities|FlowControl|Sequence
        (:then_0
          (bind _outhit (Collision|LineTraceByChannel _returnvalue (+ _returnvalue (* (Math|Vector|GetForwardVector _arrow) 2e+03)) "TraceTypeQuery1" false 0 "None"))
          (if (not (Utilities|Operators|EqualEqual (.Location (Collision|BreakHitResult _outhit)) (Math|Vector|VectorZero) 0.0))
            (bind _output_get (Variables|Default|SetPoint%20B (.Location (Collision|BreakHitResult _outhit))))
            (for _array_element (Utilities|Array|MakeArray "0, 0, 0" _output_get)
              (Rendering|Debug|DrawDebugPoint _array_element 2e+01 "(R=1.000000,G=0.912680,B=0.028845,A=1.000000)" 0.0))
            (Rendering|Debug|DrawDebugLine (Variables|Default|GetPoint%20A) (Variables|Default|GetPoint%20B) "(R=1.000000,G=0.019947,B=0.059748,A=1.000000)" 0.0 1.0)))
        (:then_1
          (Transformation|SetWorldLocation _distance (+ (* (+ _point_a (Variables|Default|GetPoint%20B)) 0.5) "0.000000,0.000000,15.000000") false false)
          (Rendering|Components|TextRender|SetText _distance (Utilities|Text|ToText(Float) (/ (Math|Vector|Distance(Vector) _point_a (Variables|Default|GetPoint%20B)) 5.0) "HalfToEven")) ; This actually sets the text for the distance.
          (bind _returnvalue_2 (Actor|GetActorOfClass "/Game/Lab0/LearningStops/BP_Learning_Stops.BP_Learning_Stops_C")) ; This whole stretch up to the "Tape Measure Used" is for the tutorial.
          (bind _returnvalue_3 (Game|GetCurrentLevelName true))
          (if (Utilities|Enum|Equal(Enum) _returnvalue_3 "Lab_0_Level")
            (Variables|/Game/Lab0/LearningStops/BP_Learning_Stops.BP_Learning_Stops_C|SetbTapeMeasureUsed _returnvalue_2 true)))))))

(fn ConstructionScript)