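; Manager Blueprint that links dig stakes with string in VR, using each stake's cable component.
; With no active stake, an interaction stores the stake, shows its cable and attaches the end to the VR pawn's right-hand socket.
; The next interaction moves that end to the new stake's ring mesh and clears the active stake.
; A separate event toggles the string-to-hand flag; the save-connection event is an empty stub.
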(event Custom|Set%20bStringFromStakeToHand%20Event
  ;[1 1 1] BP_StakeZ tells us to change the boolean.
  (Variables|Default|SetbStringFromStakeToHand (not (Variables|Default|GetbStringFromStakeToHand))) ; Flip the current value (NOT)
)

(event Custom|Save%20Stake%20Event
  (params (NewParam :type BP%20Stake%20Z%20Object%20Reference))
  ;[1 1 1] This is where we store the connections between stakes
)

(event Custom|Handle%20Stake%20Interaction
  (params (NewStake :type BP%20Stake%20Z%20Object%20Reference))
  ;[1 1 1] Handle the Stake Interaction
  (Variables|Default|SetNew%20Stake NewStake)
  (if (Utilities|IsValid (Variables|Default|GetCurrentStake)) ; False means no active stake/string.
    (bind _newparam (Default|GetCableComponent (Variables|Default|GetCurrentStake)))
    (Class|CableComponent|SetAttachEndtoComponent _newparam (Variables|/Game/Digging/Tools/Stake/BP_StakeZ.BP_StakeZ_C|GetRingMeshComponent (Variables|Default|GetNew%20Stake)) "None")
    (Variables|Default|SetCurrentStake 0)
    (else
      (Variables|Default|SetCurrentStake (Variables|Default|GetNew%20Stake))
      (bind _returnvalue (Actor|GetActorOfClass "/Game/VRTemplate/Blueprints/VRPawn.VRPawn_C"))
      (bind _newparam_2 (Default|GetCableComponent (Variables|Default|GetNew%20Stake)))
      (Class|CableComponent|SetAttachEndtoComponent _newparam_2 (Variables|/Game/VRTemplate/Blueprints/VRPawn.VRPawn_C|GetHandRight _returnvalue) "string_socket")
      (Rendering|SetVisibility _newparam_2 true false))))

(event EventBeginPlay)

(event Collision|EventActorBeginOverlap
  (params (OtherActor :type Actor%20Object%20Reference)))

(event EventTick
  (params (DeltaSeconds :type Float%20%28single-precision%29)))

(fn ConstructionScript)