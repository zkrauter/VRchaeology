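; VR stake in the digging tools that the player can tie string to.
; On BeginPlay it finds or spawns the shared BP_StakeConnectionManager, and its Box tracks when a BP_String overlaps it.
; While inside, right trigger shows the ring mesh and, if the VRPawn has string attached, delegates to the manager; the detach action has the manager delete the connecting string.
; Older cable-spawning logic remains as unreachable, broken leftovers.
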(event OnComponentBeginOverlap(Box)
  (params (OverlappedComponent :type Primitive%20Component%20Object%20Reference) (OtherActor :type Actor%20Object%20Reference) (OtherComp :type Primitive%20Component%20Object%20Reference) (OtherBodyIndex :type Integer) (bFromSweep :type Boolean) (SweepResult :type Hit%20Result%20Structure%20%28by%20ref%29))
  (Utilities|Casting|CastToBP_String OtherActor)
  (Variables|Default|SetbInsideStakeCollisionZone true))

(event OnComponentEndOverlap(Box)
  (params (OverlappedComponent :type Primitive%20Component%20Object%20Reference) (OtherActor :type Actor%20Object%20Reference) (OtherComp :type Primitive%20Component%20Object%20Reference) (OtherBodyIndex :type Integer))
  (Utilities|Casting|CastToBP_String OtherActor)
  (Variables|Default|SetbInsideStakeCollisionZone false))

(event Input|EnhancedActionEvents|EnhancedInputActionDetachConnectedStringAction
  (params (ActionValue :type Boolean) (ElapsedSeconds :type Float%20%28double-precision%29) (TriggeredSeconds :type Float%20%28double-precision%29) (InputAction :type Input%20Action%20Object%20Reference :default "/Game/Digging/Tools/String/DetachConnectedStringAction.DetachConnectedStringAction"))
  ;[1 1 1] Delete Connected Stake-String if Unequiping String
  (if (Variables|Default|GetbInsideStakeCollisionZone) ; Check if string in player hand is inside the stake collision zone.
    (Default|DeleteStringConnectingStakes (Variables|Default|GetConnectionManager) self)))

(event Input|EnhancedActionEvents|EnhancedInputActionIA_Right_Trigger
  (params (ActionValue :type Boolean) (ElapsedSeconds :type Float%20%28double-precision%29) (TriggeredSeconds :type Float%20%28double-precision%29) (InputAction :type Input%20Action%20Object%20Reference :default "/Game/VRTemplate/Input/Actions/IA_Right_Trigger.IA_Right_Trigger"))
  ;[1 1 1] String & Stake Functionality
  (if (Variables|Default|GetbInsideStakeCollisionZone) ; Check if string in player hand is inside the stake collision zone.
    (Rendering|SetVisibility (Variables|Default|GetRingMeshComponent) true false) ; Show the string on the stake.
    (bind _returnvalue (Actor|GetActorOfClass "/Game/VRTemplate/Blueprints/VRPawn.VRPawn_C")) ; Get the VRPawn to get the player hand.
    (if (Variables|/Game/VRTemplate/Blueprints/VRPawn.VRPawn_C|GetbIsStringAttached _returnvalue) ; Does the player have the string out.
      (Default|HandleStakeInteraction (Variables|Default|GetConnectionManager) self) ; BP_Stake_Connection_Manager handles functionality
    )))

(event EventBeginPlay
  (Input|EnableInput (Game|GetPlayerController 0))
  (bind _outactors (Actor|GetAllActorsOfClass "/Game/Digging/Tools/Stake/BP_StakeConnectionManager.BP_StakeConnectionManager_C"))
  (if (== (Utilities|Array|Length _outactors) 0)
    (bind _returnvalue (Game|SpawnActorfromClass "/Game/Digging/Tools/Stake/BP_StakeConnectionManager.BP_StakeConnectionManager_C" (Math|Transform|MakeTransform "0, 0, 0" "0, 0, 0" "1.000000,1.000000,1.000000") "Undefined" "MultiplyWithRoot" 0 0))
    (Variables|Default|SetConnectionManager _returnvalue)
    (else
      (Variables|Default|SetConnectionManager (Utilities|Array|Get(acopy) _outactors)))))

(event Collision|EventActorBeginOverlap
  (params (OtherActor :type Actor%20Object%20Reference)))

(fn ConstructionScript)

(fn GetCableComponent
  (return (Variables|Default|GetCable)))