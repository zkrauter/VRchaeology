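; A digging-tool stake that lets the VR player start a string line from it.
; Box overlaps with BP_String track whether string is in the stake's zone; right-trigger input there reveals the ring mesh.
; If the VRPawn has string attached, the first such press spawns a rope-material CableActor at the ring, its end attached to the right hand's string socket.
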(event OnComponentBeginOverlap(Box)
  (params (OverlappedComponent :type Primitive%20Component%20Object%20Reference) (OtherActor :type Actor%20Object%20Reference) (OtherComp :type Primitive%20Component%20Object%20Reference) (OtherBodyIndex :type Integer) (bFromSweep :type Boolean) (SweepResult :type Hit%20Result%20Structure%20%28by%20ref%29))
  (Utilities|Casting|CastToBP_String OtherActor)
  (Variables|Default|SetbInsideStakeCollisionZone true)
  (Development|PrintString "String within Collision Box"))

(event OnComponentEndOverlap(Box)
  (params (OverlappedComponent :type Primitive%20Component%20Object%20Reference) (OtherActor :type Actor%20Object%20Reference) (OtherComp :type Primitive%20Component%20Object%20Reference) (OtherBodyIndex :type Integer))
  (Utilities|Casting|CastToBP_String OtherActor)
  (Variables|Default|SetbInsideStakeCollisionZone false)
  (Development|PrintString "OUT"))

(event Input|EnhancedActionEvents|EnhancedInputActionIA_Right_Trigger
  (params (ActionValue :type Boolean) (ElapsedSeconds :type Float%20%28double-precision%29) (TriggeredSeconds :type Float%20%28double-precision%29) (InputAction :type Input%20Action%20Object%20Reference :default "/Game/VRTemplate/Input/Actions/IA_Right_Trigger.IA_Right_Trigger"))
  (if (Variables|Default|GetbInsideStakeCollisionZone)
    (Rendering|SetVisibility (Variables|Default|GetRingMeshComponent) true false)
    ;[1 1 1] Comment
    (bind _returnvalue (Actor|GetActorOfClass "/Game/VRTemplate/Blueprints/VRPawn.VRPawn_C"))
    (if (Variables|/Game/VRTemplate/Blueprints/VRPawn.VRPawn_C|GetbIsStringAttached _returnvalue)
      (Development|PrintString (Utilities|String|ToString(Boolean) (Variables|Default|GethasSpawned)) true true "(R=0.135417,G=0.000000,B=0.100110,A=1.000000)" 25.0)
      (if (not (Variables|Default|GethasSpawned))
        (bind _returnvalue_2 (Game|SpawnActorfromClass "/Script/CableComponent.CableActor" (Math|Transform|MakeTransform (Transformation|GetWorldLocation (Variables|Default|GetRingMeshComponent)) "0, 0, 0" "0.100000,0.100000,0.100000") "Undefined" "MultiplyWithRoot" 0 0))
        (Variables|Default|SethasSpawned true)
        (Rendering|Material|SetMaterial (Variables|/Script/CableComponent.CableActor|GetCableComponent _returnvalue_2) 0 "/Game/Digging/Tools/String/Rope.Rope")
        (Class|CableComponent|SetAttachEndtoComponent (Variables|/Script/CableComponent.CableActor|GetCableComponent _returnvalue_2) (Variables|/Game/VRTemplate/Blueprints/VRPawn.VRPawn_C|GetHandRight _returnvalue) "string_socket") ; Attaches cable to right hand socket
        (Variables|/Script/CableComponent.CableComponent|SetCableLength (Variables|/Script/CableComponent.CableActor|GetCableComponent _returnvalue_2) 1.0)
        (Variables|/Script/CableComponent.CableComponent|SetbEnableStiffness (Variables|/Script/CableComponent.CableActor|GetCableComponent _returnvalue_2) true)))))

(event EventBeginPlay
  (Input|EnableInput (Game|GetPlayerController 0)))

(event Collision|EventActorBeginOverlap
  (params (OtherActor :type Actor%20Object%20Reference)))

(fn ConstructionScript
  (|CallParentFunction))