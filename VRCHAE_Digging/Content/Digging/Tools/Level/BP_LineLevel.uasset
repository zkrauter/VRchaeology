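; BP_LineLevel is a line level tool for digging whose bubble shows whether it sits level.
; BeginPlay attaches the bubble to a mesh socket and, in Lab_0_Level, sets LevelUsed on BP_Learning_Stops for tutorial Stop 3.
; Each Tick maps the level's world roll to a clamped bubble Y offset.
; The level glows red unless that offset is near centre.
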(event EventBeginPlay
  (Transformation|AttachComponentToComponent (Variables|Default|GetBubble) (Variables|Default|GetLineLevel) "bubble_socket" "KeepRelative" "KeepRelative" "KeepRelative" true) ; Fixes the bubble onto the Line Level.
  (bind _returnvalue (Actor|GetActorOfClass "/Game/Lab0/LearningStops/BP_Learning_Stops.BP_Learning_Stops_C")) ; This whole stretch up to the "Level Used" is for the tutorial.
  (bind _returnvalue_2 (Game|GetCurrentLevelName true))
  (if (Utilities|Enum|Equal(Enum) _returnvalue_2 "Lab_0_Level")
    (Variables|/Game/Lab0/LearningStops/BP_Learning_Stops.BP_Learning_Stops_C|SetbLevelUsed _returnvalue true) ; Solely for Stop 3.
  ))

(event Collision|EventActorBeginOverlap
  (params (OtherActor :type Actor%20Object%20Reference)))

(event EventTick
  (params (DeltaSeconds :type Float%20%28single-precision%29))
  (bind _linelevel (Variables|Default|GetLineLevel))
  (bind _returnvalue (Transformation|GetWorldRotation _linelevel))
  (bind _roll (Math|Rotator|BreakRotator _returnvalue))
  (bind _returnvalue_2 (Math|Float|MapRangeClamped _roll -45.0 45.0 -1.5e+03 1.5e+03))
  ;[1 1 1] Line Level Functionality
  (Transformation|SetRelativeLocation (Variables|Default|GetBubble) (Math|Vector|MakeVector 0.0 _returnvalue_2 0.0) false false) ; Moving the bubble accordingly.
  (if (and (<= _returnvalue_2 1.5e+02) (>= _returnvalue_2 -1.5e+02)) ; True -> No glow. False -> Glow red.
    (Rendering|Material|SetMaterial (Variables|Default|GetLineLevel) 0 "/Game/Digging/Tools/Level/Material_002.Material_002")
    (else
      (Rendering|Material|SetMaterial (Variables|Default|GetLineLevel) 0 "/Game/Digging/Tools/Level/Glow_Red_Material.Glow_Red_Material"))))

(fn ConstructionScript)