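; Spawner for the small diggable cubes, currently set up to fill the tutorial level's crate through the Level0CrateSpawner event, as BeginPlay is empty.
; The event spawns a reference BP_SmallCube to read its scale, then lays a single-layer grid from the crate's start position, stepping negatively in X and Y.
; CanSpawnCube checks the shared ExcavatedBlocks set, held here to avoid per-cube copies, to reject previously occupied locations.
; Older test grid loops remain disconnected.
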(event Custom|Level%200%20Crate%20Spawner
  ;[1 1 1] Current setup of the block spawning
  (bind _returnvalue (Game|SpawnActorfromClass "/Game/Digging/Ground/BP_SmallCube.BP_SmallCube_C" (Math|Transform|MakeTransform (Math|Vector|MakeVector 0.0 0.0 0.0) "0, 0, 0" "0.020000,0.020000,0.020000") "Undefined" "MultiplyWithRoot" 0 0)) ; Spawned since we need a reference. First cube is hidden under the map. The rest is inside the crate in the tutorial
  (Variables|Default|SetCubeScale (Variables|/Game/Digging/Ground/BP_SmallCube.BP_SmallCube_C|GetCubeScale _returnvalue))
  (Variables|Default|SetCubeScaleToDistance (* (* (Variables|/Game/Digging/Ground/BP_SmallCube.BP_SmallCube_C|GetCubeScale _returnvalue) 1e+02) -1.0))
  (Variables|Default|SetCurrentXLocation (Variables|Default|GetCrateXStart))
  (Variables|Default|SetCurrentYLocation (Variables|Default|GetCrateYStart))
  (for _index (range 0 63) ; Run for X of cube grid
    (Variables|Default|SetCurrentXLocation (+ (Variables|Default|GetCubeScaleToDistance) (Variables|Default|GetCurrentXLocation)))
    (for _index_2 (range 0 39) ; Run for Y of cube grid
      (Game|SpawnActorfromClass "/Game/Digging/Ground/BP_SmallCube.BP_SmallCube_C" (Math|Transform|MakeTransform (Math|Vector|MakeVector (Variables|Default|GetCurrentXLocation) (Variables|Default|GetCurrentYLocation) (Variables|Default|GetCrateZStart)) "0, 0, 0" "0.020000,0.020000,0.020000") "Undefined" "MultiplyWithRoot" 0 0)
      (Variables|Default|SetCurrentYLocation (+ (Variables|Default|GetCubeScaleToDistance) (Variables|Default|GetCurrentYLocation))))
    (Variables|Default|SetCurrentYLocation (Variables|Default|GetCrateYStart))))

(event EventBeginPlay
  ;[1 1 1] Current setup of the block spawning
)

(fn ConstructionScript)

(fn CanSpawnCube
  ;[1 1 1] WE NEEDED TO MAKE THIS IN BLOCKSPAWNER BECAUSE IF WE DID THIS IN SMALLCUBE, IT WOULD MAKE A NEW VECTOR LIST EVERY TIME
  (Variables|Default|SetCanSpawn (not (Utilities|Set|Contains (Variables|Default|GetExcavatedBlocks) (Variables|Default|GetLocation)))))