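; BP_POI is a glowing point-of-interest actor that starts a learning stop when the VR player stays near it.
; Entering its trigger radius notifies BP_Learning_Stops of the overlap and plays a timeline that fades the glow, activating the stop only at zero intensity.
; Leaving reverses the fade to restore the glow.
; Both overlap handlers skip their work while a stop is active, preventing concurrent stops.
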(event OnComponentBeginOverlap(GlowLightTriggerRadius)
  (params (OverlappedComponent :type Primitive%20Component%20Object%20Reference) (OtherActor :type Actor%20Object%20Reference) (OtherComp :type Primitive%20Component%20Object%20Reference) (OtherBodyIndex :type Integer) (bFromSweep :type Boolean) (SweepResult :type Hit%20Result%20Structure%20%28by%20ref%29))
  (Utilities|Casting|CastToVRPawn OtherActor)
  (bind _returnvalue (Actor|GetActorOfClass "/Game/Lab0/LearningStops/BP_Learning_Stops.BP_Learning_Stops_C"))
  (if (not (Variables|/Game/Lab0/LearningStops/BP_Learning_Stops.BP_Learning_Stops_C|GetbIsStopActive _returnvalue)) ; Don't allow multiple concurrent Stops
    (Default|POIOverlap _returnvalue) ; Checks what POI we are overlapping in BP_Learning_Stops
    (bind _fadeglowtimelinetrack (Timeline|FadeGlowTimeline Play)
      (:Update
        (Rendering|Components|Light|SetIntensity (Variables|Default|GetGlowLight) (* _fadeglowtimelinetrack (Variables|Default|GetGlowLightIntensity))))
      (:Finished
        (if (== (* _fadeglowtimelinetrack (Variables|Default|GetGlowLightIntensity)) 0.0) ; Activate a Stop only if the Fade has fully finished
          (bind _returnvalue_2 (Actor|GetActorOfClass "/Game/Lab0/LearningStops/BP_Learning_Stops.BP_Learning_Stops_C"))
          (Default|ActivateStop _returnvalue_2))))))

(event OnComponentEndOverlap(GlowLightTriggerRadius)
  (params (OverlappedComponent :type Primitive%20Component%20Object%20Reference) (OtherActor :type Actor%20Object%20Reference) (OtherComp :type Primitive%20Component%20Object%20Reference) (OtherBodyIndex :type Integer))
  (Utilities|Casting|CastToVRPawn OtherActor)
  (bind _returnvalue (Actor|GetActorOfClass "/Game/Lab0/LearningStops/BP_Learning_Stops.BP_Learning_Stops_C"))
  (if (not (Variables|/Game/Lab0/LearningStops/BP_Learning_Stops.BP_Learning_Stops_C|GetbIsStopActive _returnvalue)) ; Don't allow the glow to reverse during a stop
    (bind _fadeglowtimelinetrack (Timeline|FadeGlowTimeline Reverse)
      (:Update
        (Rendering|Components|Light|SetIntensity (Variables|Default|GetGlowLight) (* _fadeglowtimelinetrack (Variables|Default|GetGlowLightIntensity))))
      (:Finished
        (if (== (* _fadeglowtimelinetrack (Variables|Default|GetGlowLightIntensity)) 0.0) ; Activate a Stop only if the Fade has fully finished
          (bind _returnvalue_2 (Actor|GetActorOfClass "/Game/Lab0/LearningStops/BP_Learning_Stops.BP_Learning_Stops_C"))
          (Default|ActivateStop _returnvalue_2))))))

(event EventBeginPlay)

(event Collision|EventActorBeginOverlap
  (params (OtherActor :type Actor%20Object%20Reference)))

(event EventTick
  (params (DeltaSeconds :type Float%20%28single-precision%29)))

(fn ConstructionScript)