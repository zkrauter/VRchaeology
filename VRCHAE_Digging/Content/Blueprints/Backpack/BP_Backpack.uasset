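; BP_Backpack is a briefcase-style backpack that opens or closes each time its GrabComponent is grabbed, giving access to inventory slots.
; Open and Close timelines lerp the BriefcaseBottomFoam yaw between the closed and open angles, then update IsOpen when finished.
; Inventory slots start hidden and are shown after opening and hidden after closing by toggling the Top component's visibility with propagation to its children.
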(event OnGrabbed(GrabComponent)
  (if (Variables|Default|GetisOpen)
    (CallFunction|CloseBackpack)
    (else
      (CallFunction|OpenBackpack))))

(event Custom|openBackpack
  (bind _angle (Timeline|Open PlayFromStart)
    (:Update
      (Transformation|SetRelativeRotation (Variables|Default|GetBriefcase_Bottom_Foam) (Math|Rotator|MakeRotator 0.0 0.0 (Math|Float|Lerp (Variables|Default|GetcloseAngle) (Variables|Default|GetopenAngle) _angle)) false false))
    (:Finished
      (Variables|Default|SetisOpen true)
      (CallFunction|ShowInventorySlots))))

(event Custom|closeBackpack
  (bind _angle (Timeline|Close PlayFromStart)
    (:Update
      (Transformation|SetRelativeRotation (Variables|Default|GetBriefcase_Bottom_Foam) (Math|Rotator|MakeRotator 0.0 0.0 (Math|Float|Lerp (Variables|Default|GetopenAngle) (Variables|Default|GetcloseAngle) _angle)) false false))
    (:Finished
      (Variables|Default|SetisOpen false)
      (CallFunction|HideInventorySlots))))

(event EventBeginPlay
  (CallFunction|HideInventorySlots))

(event Collision|EventActorBeginOverlap
  (params (OtherActor :type Actor%20Object%20Reference)))

(event EventTick
  (params (DeltaSeconds :type Float%20%28single-precision%29)))

(fn ConstructionScript)

(fn ToggleBackpack
  (if (Variables|Default|GetisOpen)
    (CallFunction|CloseBackpack)
    (else
      (CallFunction|OpenBackpack))))

(fn CheckHeld
  (params (hand :type Grab%20Component%20Object%20Reference))
  (if (== hand (Variables|BP_Backpack_C|GetGrabComponent self))
    (return true)
    (else
      (return false))))

(fn ShowInventorySlots
  (Rendering|SetVisibility (Variables|Default|GetTop) true true))

(fn HideInventorySlots
  (Rendering|SetVisibility (Variables|Default|GetTop) false true))