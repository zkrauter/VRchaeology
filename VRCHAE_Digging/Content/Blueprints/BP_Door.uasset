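; BP_Door is a door that a motion controller can grab and swing open or closed.
; Grab stores the controller as Hand when it is within the handle's collision sphere, and Release clears it if it matches.
; On Tick, the door's world yaw follows the hand through an offset look-at rotation clamped to a half-turn range.
; When not held, it snaps to zero rotation if nearly closed.
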(event EventTick
  (params (DeltaSeconds :type Float%20%28single-precision%29))
  (bind _hand (Variables|Default|GetHand))
  (bind _doorbody (Variables|Default|GetDoorBody))
  ;[1 1 1] Set Door Rotation
  (Utilities|IsValid _hand
    (:Is%20Valid
      (Transformation|SetWorldRotation (Variables|Default|GetDoorBody) (Math|Rotator|MakeRotator 0.0 0.0 (Math|Float|ClampAngle (- (.yaw (Math|Rotator|FindLookatRotation (Transformation|GetWorldLocation _hand) (Transformation|GetWorldLocation _doorbody))) -9e+01) -9e+01 9e+01)) false false))
    (:Is%20Not%20Valid
      (if (Math|Float|NearlyEqual(Float) (.yaw (Transformation|GetWorldRotation _doorbody)) 0.0 1e+01)
        (Transformation|SetWorldRotation (Variables|Default|GetDoorBody) "0, 0, 0" false false)))))

(event EventGrab
  (params (MotionController :type Motion%20Controller%20Component%20Object%20Reference))
  (bind _handlecollision (Variables|Default|GetHandleCollision))
  (if (Utilities|Operators|EqualEqual (Transformation|GetWorldLocation MotionController) (Transformation|GetWorldLocation _handlecollision) (Variables|/Script/Engine.SphereComponent|GetSphereRadius _handlecollision))
    (Variables|Default|SetHand MotionController)))

(event EventRelease
  (params (MotionController :type Motion%20Controller%20Component%20Object%20Reference))
  (if (== MotionController (Variables|Default|GetHand))
    (Variables|Default|SetHand 0)))

(fn ConstructionScript)